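; Score actor for a pinball-style game that tracks the player's score and remaining balls.
; Functions add points for bumper hits and relaunches, and add or remove balls.
; Bumper hits also copy the score into the PersistantData game instance, while relaunch points are not copied there directly.
; Tick checks the ball count every frame and opens the GameOver level once none remain.
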(event Collision|EventActorBeginOverlap
  (params (OtherActor :type Actor%20Object%20Reference)))

(event EventTick
  (params (DeltaSeconds :type Float%20%28single-precision%29))
  (if (<= (Variables|Default|GetBalls%20Left) 0)
    (Game|OpenLevel(byName) "GameOver")))

(fn ConstructionScript)

(fn BumperHit
  (bind _output_get (Variables|Default|SetScore (+ (Variables|Default|GetScore) 10)))
  (bind _aspersistant_data (Utilities|Casting|CastToPersistantData (Game|GetGameInstance)))
  (Variables|/Game/Blueprints/Objects/PersistantData.PersistantData_C|SetScore _aspersistant_data _output_get))

(fn ReLaunch
  (Variables|Default|SetScore (+ (Variables|Default|GetScore) 50)))

(fn ExtraBall
  (Variables|Default|SetBalls%20Left (+ (Variables|Default|GetBalls%20Left) 1)))

(fn LoseBall
  (Variables|Default|SetBalls%20Left (- (Variables|Default|GetBalls%20Left) 1)))