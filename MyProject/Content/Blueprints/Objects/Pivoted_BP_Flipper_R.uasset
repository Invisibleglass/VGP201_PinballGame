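; Right-hand flipper actor, likely for a pinball-style game, that swings while Right Shift is held and returns on release.
; Press and release set opposite signed speeds and a Rotate flag, with player 0 input enabled at BeginPlay.
; Tick rolls the Arrow component, used as the pivot, by speed times delta time.
; At either 30-degree limit it stops and snaps just inside, so the next swing can start.
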(event EventBeginPlay
  (Input|EnableInput (Game|GetPlayerController 0)))

(event Collision|EventActorBeginOverlap
  (params (OtherActor :type Actor%20Object%20Reference)))

(event EventTick
  (params (DeltaSeconds :type Float%20%28single-precision%29))
  (bind _arrow (Variables|Default|GetArrow))
  (bind _relativerotation (Variables|/Script/Engine.SceneComponent|GetRelativeRotation _arrow))
  (bind _roll (Math|Rotator|BreakRotator _relativerotation))
  (if (Variables|Default|GetRotate)
    (if (or (>= _roll 3e+01) (<= _roll -3e+01))
      (Variables|Default|SetRotate false)
      (CallFunction|ResetRotation)
      (else
        (Transformation|AddRelativeRotation (Variables|Default|GetArrow) (Math|Rotator|MakeRotator (* DeltaSeconds (Variables|Default|GetSpeed)) 0.0 0.0) false false)))))

(event Input|KeyboardEvents|RightShift
  (params (Key :type Key%20Structure))
  (:Pressed
    (CallFunction|RotateUp))
  (:Released
    (CallFunction|RotateDown)))

(fn ConstructionScript)

(fn RotateUp
  (Variables|Default|SetRotate true)
  (Variables|Default|SetSpeed -4e+02))

(fn RotateDown
  (Variables|Default|SetRotate true)
  (Variables|Default|SetSpeed 4e+02))

(fn ResetRotation
  (bind _arrow (Variables|Default|GetArrow))
  (bind _arrow_2 (Variables|Default|GetArrow))
  (bind _relativerotation (Variables|/Script/Engine.SceneComponent|GetRelativeRotation _arrow_2))
  (bind _roll (Math|Rotator|BreakRotator _relativerotation))
  (if (>= _roll 3e+01)
    (Transformation|SetRelativeRotation _arrow "0.000000,0.000000,29.900000" false false)
    (elif (<= _roll -3e+01)
      (Transformation|SetRelativeRotation _arrow "0.000000,0.000000,-29.900000" false false))))