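; BP_Ball is a physics ball actor that takes keyboard input from player controller 0.
; Holding Space overrides the Sphere component's mass to very heavy, and releasing it makes it very light.
; Pressing Space also repositions BallMesh if it lies near a hardcoded world point.
; R calls ResetBall, which zeroes BallMesh's velocity and sets its relative location to the actor's world location.
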(event EventBeginPlay
  (Input|EnableInput (Game|GetPlayerController 0)))

(event Collision|EventHit
  (params (MyComp :type Primitive%20Component%20Object%20Reference) (Other :type Actor%20Object%20Reference) (OtherComp :type Primitive%20Component%20Object%20Reference) (bSelfMoved :type Boolean) (HitLocation :type Vector :default "0, 0, 0") (HitNormal :type Vector :default "0, 0, 0") (NormalImpulse :type Vector :default "0, 0, 0") (Hit :type Hit%20Result%20Structure%20%28by%20ref%29)))

(event Input|KeyboardEvents|SpaceBar
  (params (Key :type Key%20Structure :default "None"))
  (bind _sphere (Variables|Default|GetSphere))
  (:Pressed
    (Class|PrimitiveComponent|SetMassOverrideinKg _sphere "None" 5e+04 true)
    (if (Utilities|Operators|EqualEqual (Transformation|GetWorldLocation (Variables|Default|GetBallMesh)) "1470.000000,-840.000000,520.000000" 1e+01)
      (Transformation|SetRelativeLocation (Variables|Default|GetBallMesh) (Transformation|GetActorLocation) false false)))
  (:Released
    (Class|PrimitiveComponent|SetMassOverrideinKg _sphere "None" 0.1 true)))

(event Input|KeyboardEvents|R
  (params (Key :type Key%20Structure :default "None"))
  (:Pressed
    (CallFunction|ResetBall)))

(fn ConstructionScript)

(fn ResetBall
  (Class|PrimitiveComponent|SetAllPhysicsLinearVelocity (Variables|Default|GetBallMesh) "0, 0, 0" false)
  (Transformation|SetRelativeLocation (Variables|Default|GetBallMesh) (Transformation|GetActorLocation) false false))